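; AI controller that drives an AI_PlayerBP pawn along a randomly chosen TrackSplineBP, picked shortly after BeginPlay.
; Tick derives a travel duration from spline length and the pawn's max walk speed, and repeatedly calls the delayed Run event.
; Run scales the Move timeline's play rate by that duration, and each update issues MoveToLocation to the interpolated distance along the spline.
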(event `self.ReceiveBeginPlay`
  (`KismetSystemLibrary.Delay` 0.2)
  (`|ExecutionSequence`
    (:`then_0`
      (bind _outactors (`GameplayStatics.GetAllActorsOfClass` "/Game/Blueprints/TrackSplineBP.TrackSplineBP_C"))
      (set `self.Spline ` (`KismetArrayLibrary.Array_Random` _outactors)))
    (:`then_1`
      (set `self.Condition` true))))

(event `self.ReceiveTick`
  (params (DeltaSeconds :type "Float (single-precision)"))
  (if (`self.Condition`)
    (`self.Run`)
    (bind _asai_player_bp (cast `/Game/Blueprints/AI_PlayerBP` (`self.K2_GetPawn`)))
    (set `self.Durration` (/ (`SplineComponent.GetSplineLength` (`/Game/Blueprints/TrackSplineBP.Spline Path` (`self.Spline `))) (`CharacterMovementComponent.MaxWalkSpeed` (`Character.CharacterMovement` _asai_player_bp))))))

(event `Run`
  (bind _spline_path (`/Game/Blueprints/TrackSplineBP.Spline Path` (`self.Spline `)))
  (`KismetSystemLibrary.Delay` 1.0)
  (`TimelineComponent.SetPlayRate` (`self.Move`) (/ 1.0 (`self.Durration`)))
  (bind (_direction _alpha) (`Timeline|Move`)
    (:`Update`
      (set `self.Alpha` _alpha)
      (`self.MoveToLocation` (`SplineComponent.GetLocationAtDistanceAlongSpline` _spline_path (`KismetMathLibrary.Lerp` 0.0 (`SplineComponent.GetSplineLength` _spline_path) (`self.Alpha`)) "World") -1.0 true true false true null))))

(fn `UserConstructionScript`)