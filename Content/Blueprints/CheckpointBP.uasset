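; Race checkpoint actor that tracks checkpoint and lap progress for PlayerBP and AI_PlayerBP racers.
; FrontBox overlap sets the racer's checkpoint to this index, or at a lap point resets it, increments the lap and teleports the racer.
; BackBox overlap decrements the checkpoint when it exceeds this index.
; The construction script derives the index from the object name unless a custom one is used, and sets plane visibility.
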(event `self.BackBox.OnComponentBeginOverlap`
  (params (OverlappedComponent :type "PrimitiveComponent Object Reference") (OtherActor :type "Actor Object Reference") (OtherComp :type "PrimitiveComponent Object Reference") (OtherBodyIndex :type Integer) (bFromSweep :type Boolean) (SweepResult :type "HitResult Structure (by ref)"))
  (`|ExecutionSequence`
    (:`then_0`
      (bind _asplayer_bp (cast `/Game/Blueprints/PlayerBP` OtherActor))
      (bind _checkpoint (`/Game/Blueprints/PlayerBP.Checkpoint` _asplayer_bp))
      (if (> _checkpoint (`self.Checkpoint Index`))
        (set `/Game/Blueprints/PlayerBP.Checkpoint` (- _checkpoint 1) _asplayer_bp)))
    (:`then_1`
      (bind _asai_player_bp (cast `/Game/Blueprints/AI_PlayerBP` OtherActor))
      (bind _checkpoint_2 (`/Game/Blueprints/AI_PlayerBP.Checkpoint` _asai_player_bp))
      (if (> _checkpoint_2 (`self.Checkpoint Index`))
        (set `/Game/Blueprints/AI_PlayerBP.Checkpoint` (- _checkpoint_2 1) _asai_player_bp)))))

(event `self.FrontBox.OnComponentBeginOverlap`
  (params (OverlappedComponent :type "PrimitiveComponent Object Reference") (OtherActor :type "Actor Object Reference") (OtherComp :type "PrimitiveComponent Object Reference") (OtherBodyIndex :type Integer) (bFromSweep :type Boolean) (SweepResult :type "HitResult Structure (by ref)"))
  (bind _lap_teleportation_point (`self.Lap Teleportation Point`))
  (if (`self.Lap Point`)
    (`|ExecutionSequence`
      (:`then_0`
        (bind _asplayer_bp (cast `/Game/Blueprints/PlayerBP` OtherActor))
        (set `/Game/Blueprints/PlayerBP.Checkpoint` 0 _asplayer_bp)
        (set `/Game/Blueprints/PlayerBP.Lap` (+ (`/Game/Blueprints/PlayerBP.Lap` _asplayer_bp) 1) _asplayer_bp)
        (`self.K2_SetActorTransform` _asplayer_bp _lap_teleportation_point false true))
      (:`then_1`
        (bind _asai_player_bp (cast `/Game/Blueprints/AI_PlayerBP` OtherActor))
        (set `/Game/Blueprints/AI_PlayerBP.Checkpoint` 0 _asai_player_bp)
        (set `/Game/Blueprints/AI_PlayerBP.Lap` (+ (`/Game/Blueprints/AI_PlayerBP.Lap` _asai_player_bp) 1) _asai_player_bp)
        (`self.K2_SetActorTransform` _asai_player_bp _lap_teleportation_point false true)))
    (else
      (`|ExecutionSequence`
        (:`then_0`
          (bind _asplayer_bp_2 (cast `/Game/Blueprints/PlayerBP` OtherActor))
          (set `/Game/Blueprints/PlayerBP.Checkpoint` (`self.Checkpoint Index`) _asplayer_bp_2))
        (:`then_1`
          (bind _asai_player_bp_2 (cast `/Game/Blueprints/AI_PlayerBP` OtherActor))
          (set `/Game/Blueprints/AI_PlayerBP.Checkpoint` (`self.Checkpoint Index`) _asai_player_bp_2))))))

(fn `UserConstructionScript`
  (if (`self.Use Custom Index?`)
    (set `self.Checkpoint Index` (`self.Checkpoint Index`))
    (else
      (set `self.Checkpoint Index` (`KismetStringLibrary.Conv_StringToInt` (`KismetStringLibrary.Replace` (`KismetSystemLibrary.GetObjectName` self) "CheckpointBP_C_")))))
  (`SceneComponent.SetVisibility` (`self.Plane`) (`self.New Visibility`) false))