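; ItemBoxBP is an item box pickup that gives a PlayerBP a new item on overlap.
; An UpAndDown timeline moves the mesh vertically while idle.
; On overlap it plays a break sound scaled by player speed, spawns an explosion effect and runs a second timeline on the mesh height.
; A DoOnce grants one item per run of that timeline, resetting when it finishes and the idle motion restarts.
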(event `self.ReceiveBeginPlay`
  (bind (_direction _newtrack_0) (`Timeline|Up and Down` :!via `PlayFromStart` :!label _label)
    (:`Update`
      (`SceneComponent.K2_SetRelativeLocation` (`self.StaticMesh`) (`KismetMathLibrary.MakeVector` 0.0 0.0 _newtrack_0) false true))))

(event `Move Up and Down`
  (goto _label :!via `PlayFromStart`))

(event `self.Sphere.OnComponentBeginOverlap`
  (params (OverlappedComponent :type "PrimitiveComponent Object Reference") (OtherActor :type "Actor Object Reference") (OtherComp :type "PrimitiveComponent Object Reference") (OtherBodyIndex :type Integer) (bFromSweep :type Boolean) (SweepResult :type "HitResult Structure (by ref)"))
  (bind (_returnvalue_location _returnvalue_rotation _returnvalue_scale) (`KismetMathLibrary.BreakTransform` (`SceneComponent.K2_GetComponentToWorld` (`self.StaticMesh`))))
  (bind _asplayer_bp (cast `/Game/Blueprints/PlayerBP` OtherActor))
  (`GameplayStatics.PlaySoundAtLocation` "/Game/SFX/ItemBox_Break.ItemBox_Break" (`self.K2_GetActorLocation`) (struct) (`KismetMathLibrary.MapRangeClamped` (`KismetMathLibrary.VSize` (`self.GetVelocity` _asplayer_bp)) 3000.0 0.0 1.0 0.05) 1.0 0.0 "/Game/SFX/SBK_SoundAttenuation.SBK_SoundAttenuation" null null null)
  (`NiagaraFunctionLibrary.SpawnSystemAtLocation` "/Game/VFX/PS_ItemBox_Explode.PS_ItemBox_Explode" _returnvalue_location _returnvalue_rotation _returnvalue_scale)
  (`TimelineComponent.Stop` (`self.Up and Down`))
  (bind (_direction _newtrack_0) (`Timeline|Timeline_0` :!via `PlayFromStart`)
    (:`Update`
      (`SceneComponent.K2_SetRelativeLocation` (`self.StaticMesh`) (`KismetMathLibrary.MakeVector` 0.0 0.0 _newtrack_0) false true)
      (`/Engine/EditorBlueprintResources/StandardMacros.DoOnce` false :!label _label_2
        (:`Completed`
          (`/Game/Blueprints/PlayerBP.Set New Item` _asplayer_bp))))
    (:`Finished`
      (`self.Move Up and Down`)
      (goto _label_2 :!via `Reset`))))

(fn `UserConstructionScript`)