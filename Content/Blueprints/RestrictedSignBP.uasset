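; Restricted sign prop that snaps its static mesh to the surface below it when constructed.
; The construction script traces downward on the Camera channel, moves the mesh to the hit point and derives pitch and roll from the surface normal, keeping yaw.
; A one-shot break sequence that hides the mesh, disables collision and spawns RestrictedSignBrokenBP is present but unconnected, and the AddImpulse event is empty.
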(event `/Game/Blueprints/BPI_Interact.Add Impulse`
  (params (`Hit Actor` :type "Actor Object Reference")))

(fn `UserConstructionScript`
  (bind _returnvalue (`self.K2_GetActorLocation`))
  (bind _staticmesh (`self.StaticMesh`))
  (bind (_returnvalue_roll _returnvalue_pitch _returnvalue_yaw) (`KismetMathLibrary.BreakRotator` (`SceneComponent.K2_GetComponentRotation` _staticmesh)))
  (bind (_outhit _returnvalue_2) (`KismetSystemLibrary.LineTraceSingle` _returnvalue (+ _returnvalue (* (`self.GetActorUpVector`) -500.0)) "TraceTypeQuery2" false (`|MakeArray` null :!type "Actor Object Reference")))
  (if _returnvalue_2
    (bind (_bblockinghit _binitialoverlap _time _distance _location _impactpoint _normal _impactnormal) (`GameplayStatics.BreakHitResult` _outhit))
    (bind (_returnvalue_roll_2 _returnvalue_pitch_2) (`KismetMathLibrary.BreakRotator` (`KismetMathLibrary.Conv_VectorToRotator` (+ _impactnormal (90.0 0.0 0.0)))))
    (`SceneComponent.K2_SetWorldLocationAndRotation` _staticmesh _impactpoint (`KismetMathLibrary.MakeRotator` _returnvalue_roll_2 _returnvalue_pitch_2 _returnvalue_yaw) false true)))