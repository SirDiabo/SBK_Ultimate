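; Firework rocket actor that explodes on nearby obstacles and stuns players it touches.
; Each tick it traces a short line ahead on the Visibility channel, and a hit spawns the explosion effect, plays a random-pitch boom and destroys the rocket.
; A separate sphere overlap calls FireworkStun on human and AI players without destroying the rocket.
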(event `self.ReceiveTick`
  (params (DeltaSeconds :type "Float (single-precision)"))
  (bind _returnvalue (`self.K2_GetActorLocation`))
  (bind (_outhit _returnvalue_2) (`KismetSystemLibrary.LineTraceSingle` _returnvalue (+ _returnvalue (* (`self.GetActorForwardVector`) 200.0)) "TraceTypeQuery1" false (`|MakeArray` null :!type "Actor Object Reference")))
  (if _returnvalue_2
    (`NiagaraFunctionLibrary.SpawnSystemAtLocation` "/Game/VFX/PS_FireworkRocket_Explosion.PS_FireworkRocket_Explosion" (`self.K2_GetActorLocation`))
    (`GameplayStatics.PlaySoundAtLocation` "/Game/SFX/FireworkRocket_Boom.FireworkRocket_Boom" (`self.K2_GetActorLocation`) (struct) 1.0 (`KismetMathLibrary.RandomFloatInRange` 0.5 1.3) 0.0 "/Game/SFX/SBK_SoundAttenuation.SBK_SoundAttenuation" null null null)
    (`self.K2_DestroyActor`)))

(event `self.Sphere.OnComponentBeginOverlap`
  (params (OverlappedComponent :type "PrimitiveComponent Object Reference") (OtherActor :type "Actor Object Reference") (OtherComp :type "PrimitiveComponent Object Reference") (OtherBodyIndex :type Integer) (bFromSweep :type Boolean) (SweepResult :type "HitResult Structure (by ref)"))
  (`|ExecutionSequence`
    (:`then_0`
      (bind _asplayer_bp (cast `/Game/Blueprints/PlayerBP` OtherActor))
      (`/Game/Blueprints/PlayerBP.Firework Stun` _asplayer_bp))
    (:`then_1`
      (bind _asai_player_bp (cast `/Game/Blueprints/AI_PlayerBP` OtherActor))
      (`/Game/Blueprints/AI_PlayerBP.Firework Stun` _asai_player_bp))))

(fn `UserConstructionScript`)