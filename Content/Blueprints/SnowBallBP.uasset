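; Snowball pawn that drives itself forward, stuns a player or AI player it overlaps, then explodes.
; On spawn, timelines grow and spin the mesh, enabling stun and collision once grown.
; Tick uses a delayed forward sphere trace to count hits, exploding with sound past MaxBounces.
; The reflection-based bounce rotation is disconnected, so hits never change its heading.
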(event `self.ReceiveBeginPlay`
  (`|ExecutionSequence` :!label _label
    (:`then_0`
      (bind (_direction _newtrack_0) (`Timeline|Grow`)
        (:`Update`
          (`SceneComponent.SetRelativeScale3D` (`self.StaticMesh`) (`KismetMathLibrary.Conv_DoubleToVector` _newtrack_0)))
        (:`Finished`
          (set `self.Can Stun` true)
          (`PrimitiveComponent.SetCollisionEnabled` (`self.StaticMesh`) "QueryAndPhysics"))))
    (:`then_1`
      (bind (_direction_2 _newtrack_0_2) (`Timeline|Spin` :!via `PlayFromStart`)
        (:`Update`
          (`SceneComponent.K2_SetRelativeRotation` (`self.StaticMesh`) (`KismetMathLibrary.MakeRotator` 0.0 _newtrack_0_2) false false))))))

(event `Spawned`
  (goto _label))

(event `self.Sphere.OnComponentBeginOverlap`
  (params (OverlappedComponent :type "PrimitiveComponent Object Reference") (OtherActor :type "Actor Object Reference") (OtherComp :type "PrimitiveComponent Object Reference") (OtherBodyIndex :type Integer) (bFromSweep :type Boolean) (SweepResult :type "HitResult Structure (by ref)"))
  (if (`self.Can Stun`)
    (`|ExecutionSequence`
      (:`then_0`
        (bind _asplayer_bp (cast `/Game/Blueprints/PlayerBP` OtherActor))
        (`/Game/Blueprints/PlayerBP.Stun Player` _asplayer_bp))
      (:`then_1`
        (bind _asai_player_bp (cast `/Game/Blueprints/AI_PlayerBP` OtherActor))
        (`/Game/Blueprints/AI_PlayerBP.Stun Player` _asai_player_bp)))
    (`NiagaraFunctionLibrary.SpawnSystemAtLocation` "/Game/VFX/PS_SnowBall_Explode.PS_SnowBall_Explode" (`self.K2_GetActorLocation`))
    (`self.K2_DestroyActor`)))

(event `self.ReceiveTick`
  (params (DeltaSeconds :type "Float (single-precision)"))
  (bind _returnvalue (`self.K2_GetActorLocation`))
  (`|ExecutionSequence`
    (:`then_0`
      (`self.AddMovementInput` (`self.GetActorForwardVector`) 1.0 true)
      (`KismetSystemLibrary.Delay` 0.2)
      (bind (_outhit _returnvalue_2) (`KismetSystemLibrary.SphereTraceSingle` _returnvalue (+ _returnvalue (* (`self.GetActorForwardVector`) 600)) 100.0 "TraceTypeQuery1" false (`|MakeArray` null :!type "Actor Object Reference")))
      (if _returnvalue_2
        (bind _result (`/Engine/EditorBlueprintResources/StandardMacros.IncrementInt` (`self.Bounce Times`))
          (:`  `
            (if (> _result (`self.Max Bounces`))
              (`NiagaraFunctionLibrary.SpawnSystemAtLocation` "/Game/VFX/PS_SnowBall_Explode.PS_SnowBall_Explode" (`self.K2_GetActorLocation`))
              (`self.K2_DestroyActor`)
              (`GameplayStatics.PlaySoundAtLocation` "/Game/SFX/Snowball_Break.Snowball_Break" (`self.K2_GetActorLocation`) (struct) 1.0 1.0 0.0 "/Game/SFX/SBK_SoundAttenuation.SBK_SoundAttenuation" null null null))))))))

(fn `UserConstructionScript`)