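; GM_SBK is a game mode that sets game input at start and tracks time elapsed since play began.
; BeginPlay records a wall-clock start time and has a loop, bounded from player count to zero, meant to set game-only input and hide cursors.
; Each Tick subtracts the start time from Now and writes the result to PlayerBP, reaching only player 0 despite the "ToEveryone" event name.
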(event `self.ReceiveBeginPlay`
  (bind (_returnvalue_year _returnvalue_month _returnvalue_day _returnvalue_hour _returnvalue_minute _returnvalue_second _returnvalue_millisecond) (`KismetMathLibrary.BreakDateTime` (`KismetMathLibrary.Now`)))
  (`|ExecutionSequence`
    (:`then_0`
      (for _index (range (`GameplayStatics.GetNumPlayerStates`) 1)
        (bind _returnvalue (`PlayerState.GetPlayerController` (`GameplayStatics.GetPlayerState` _index)))
        (`WidgetBlueprintLibrary.SetInputMode_GameOnly` _returnvalue)
        (set `PlayerController.bShowMouseCursor` false _returnvalue)))
    (:`then_1`
      (set `self.Start Time` (`KismetMathLibrary.MakeTimespan` _returnvalue_day _returnvalue_hour _returnvalue_minute _returnvalue_second _returnvalue_millisecond)))))

(event `self.ReceiveTick`
  (params (DeltaSeconds :type "Float (single-precision)"))
  (bind (_returnvalue_year _returnvalue_month _returnvalue_day _returnvalue_hour _returnvalue_minute _returnvalue_second _returnvalue_millisecond) (`KismetMathLibrary.BreakDateTime` (`KismetMathLibrary.Now`)))
  (`|ExecutionSequence`
    (:`then_0`
      (set `self.Time Since Start` (- (`KismetMathLibrary.MakeTimespan` _returnvalue_day _returnvalue_hour _returnvalue_minute _returnvalue_second _returnvalue_millisecond) (`self.Start Time`)))
      (`self.Give Passed Time Since Start to Everyone`))))

(event `Give Passed Time Since Start to Everyone`
  (bind _asplayer_bp (cast `/Game/Blueprints/PlayerBP` (`GameplayStatics.GetPlayerCharacter` 0)))
  (set `/Game/Blueprints/PlayerBP.time passed since start` (`self.Time Since Start`) _asplayer_bp))

(fn `UserConstructionScript`)